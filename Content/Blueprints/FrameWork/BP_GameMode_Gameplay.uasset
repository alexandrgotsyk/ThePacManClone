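; Gameplay game mode that sets up the gameplay camera and player control on BeginPlay.
; It spawns a CameraActor at a stored location and rotation, then makes it the player controller's view target.
; Player input is disabled, then re-enabled in the same execution chain, and BP_Player's AllowedToMove is set to true.
; A seven-second Delay before re-enabling input is disconnected and never runs.
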(event `self.ReceiveBeginPlay`
  (bind _returnvalue (`GameplayStatics.GetPlayerCharacter` 0))
  (`|ExecutionSequence`
    (:`then_6`
      ;[0 0.2604 0.02094 0.248] Gameplay Camera
      (`self.DisableInput` (`GameplayStatics.GetPlayerCharacter` 0) (`GameplayStatics.GetPlayerController` 0))
      (bind _returnvalue_2 (`|SpawnActorFromClass` "/Script/Engine.CameraActor" (`KismetMathLibrary.MakeTransform` (`self.CamGameplay_Loc`) (`self.CamGamePlay_Rot`)) "Undefined" "OverrideRootScale" null null))
      (`PlayerController.SetViewTargetWithBlend` (`GameplayStatics.GetPlayerController` 0) _returnvalue_2 0.0 "VTBlend_Linear" 0.0 false) ; Blend Time Задержка 6.8
      (`self.EnableInput` _returnvalue (`GameplayStatics.GetPlayerController` 0))
      (bind _asbp_player (cast `/Game/Blueprints/Character/BP_Player` _returnvalue))
      (set `/Game/Blueprints/Character/BP_Player.bAllowedToMove?` true _asbp_player))))

(fn `UserConstructionScript`)