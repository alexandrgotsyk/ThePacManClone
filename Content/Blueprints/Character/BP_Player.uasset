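; BP_Player is the player character, with Pac-Man-style continuous movement and a chomping animation.
; Axis inputs past a 0.7 threshold latch one of four direction flags and add movement immediately, with MoveRight setting up/down and MoveForward left/right.
; While AllowedToMove is set, Tick repeats that movement along yaw-only control axes.
; If ShouldPlayerGobble is set, Tick also toggles the open and closed meshes on a short delay.
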(event `self.ReceiveTick`
  (params (DeltaSeconds :type "Float (single-precision)"))
  (if (`self.bAllowedToMove?`)
    (`|ExecutionSequence`
      (:`then_0`
        ;[0.4688 0 0.3932] Animation Gobble
        (if (`self.bShouldPlayerGobble?`)
          (`KismetSystemLibrary.Delay` 0.2)
          (`/Engine/EditorBlueprintResources/StandardMacros.FlipFlop`
            (:`A`
              _)
            (:`B`
              _))
          (`SceneComponent.ToggleVisibility` (`self.Player_Open`) false)
          (`SceneComponent.ToggleVisibility` (`self.Player_Close`) false)))
      (:`then_1`
        (if (`self.bGoingUp?`)
          ;[1 1 1] Player Move Up/Down
          (`self.AddMovementInput` (`KismetMathLibrary.GetRightVector` (`KismetMathLibrary.MakeRotator` 0.0 0.0 (.yaw (`self.GetControlRotation`)))) (stale `InputAxis|MoveRight` _output_get) :!label _label)
          (elif (`self.bGoingDown?`)
            (`self.AddMovementInput` (`KismetMathLibrary.GetRightVector` (`KismetMathLibrary.MakeRotator` 0.0 0.0 (.yaw (`self.GetControlRotation`)))) (stale `InputAxis|MoveRight` _output_get_2) :!label _label_2)
            (elif (`self.bGoingLeft?`)
              ;[1 1 1] Player Move Right/Left
              (`self.AddMovementInput` (`KismetMathLibrary.GetForwardVector` (`KismetMathLibrary.MakeRotator` 0.0 0.0 (.yaw (`self.GetControlRotation`)))) (stale `InputAxis|MoveForward` _output_get_2) :!label _label_3)
              (elif (`self.bGoingRight?`)
                (`self.AddMovementInput` (`KismetMathLibrary.GetForwardVector` (`KismetMathLibrary.MakeRotator` 0.0 0.0 (.yaw (`self.GetControlRotation`)))) (stale `InputAxis|MoveForward` _output_get) :!label _label_4)))))))))

(event `InputAxis|MoveRight` :overrideparent false
  (params (AxisValue :type "Float (single-precision)"))
  ;[1 1 1] Player Move Up/Down
  (if (>= AxisValue 0.7)
    (set `self.bGoingLeft?` false)
    (set `self.bGoingUp?` true)
    (set `self.bGoingDown?` false)
    (set `self.bGoingRight?` false)
    (bind _output_get (set `self.InputForward` 1.0))
    (goto _label)
    (elif (<= AxisValue -0.7)
      (set `self.bGoingUp?` false)
      (set `self.bGoingDown?` true)
      (set `self.bGoingRight?` false)
      (set `self.bGoingLeft?` false)
      (bind _output_get_2 (set `self.InputForward` -1.0))
      (goto _label_2))))

(event `InputAxis|MoveForward` :overrideparent false
  (params (AxisValue :type "Float (single-precision)"))
  ;[1 1 1] Player Move Right/Left
  (if (>= AxisValue 0.7)
    (set `self.bGoingLeft?` false)
    (set `self.bGoingUp?` false)
    (set `self.bGoingDown?` false)
    (set `self.bGoingRight?` true)
    (bind _output_get (set `self.InputForward` 1.0))
    (goto _label_4)
    (elif (<= AxisValue -0.7)
      (set `self.bGoingUp?` false)
      (set `self.bGoingDown?` false)
      (set `self.bGoingRight?` false)
      (set `self.bGoingLeft?` true)
      (bind _output_get_2 (set `self.InputForward` -1.0))
      (goto _label_3))))

(fn `UserConstructionScript`)